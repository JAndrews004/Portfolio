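; Character Blueprint that manages the HUD and death screen for the player.
; BeginPlay clears existing widgets, shows MyHUD, pre-creates DeathUI and binds the HealthComp death event.
; On death, the handler swaps all widgets for DeathUI, switches input to UI only with a visible cursor, and pauses the game.
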(event Custom|HandleDeathUI
  (bind _returnvalue (Game|GetPlayerController 0))
  (bind _deathui (Variables|Default|GetDeathUI))
  ;[1 1 1] Death UI and respawn
  (Viewport|RemoveAllWidgets)
  (UserInterface|Viewport|AddtoViewport _deathui 0)
  (Input|SetInputModeUIOnly _returnvalue _deathui "DoNotLock" false)
  (Variables|/Script/Engine.PlayerController|SetbShowMouseCursor _returnvalue true)
  (Game|SetGamePaused true))

(event EventBeginPlay
  ;[1 1 1] UI
  (Viewport|RemoveAllWidgets)
  (bind _returnvalue (UserInterface|CreateWidget "/Game/UI/MyHUD.MyHUD_C"))
  (UserInterface|Viewport|AddtoViewport _returnvalue 0)
  (bind _returnvalue_2 (Game|ConstructObjectfromClass "/Game/UI/DeathUI.DeathUI_C"))
  (Variables|Default|SetDeathUI _returnvalue_2)
  ;[1 1 1] Death UI and respawn
  (EventDispatchers|BindEventtoOnDeathEvent (Variables|Default|GetHealthComp) (delegate Custom|HandleDeathUI)))

(event Collision|EventActorBeginOverlap
  (params (OtherActor :type Actor%20Object%20Reference)))

(event EventTick
  (params (DeltaSeconds :type Float%20%28single-precision%29)))

(fn ConstructionScript)