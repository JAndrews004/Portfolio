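; BP_CubeManager is an actor that saves and restores the transform and hidden state of the cubes in its TrackedCubes array.
; SaveGame writes parallel arrays into a MySaveGame object, stores it in one fixed slot and prints whether that slot exists.
; LoadGame reapplies them by TrackedCubes index, though saving skips invalid cubes, so indices can shift.
; The event graph is empty, so both functions rely on external callers.
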(event EventBeginPlay)

(event Collision|EventActorBeginOverlap
  (params (OtherActor :type Actor%20Object%20Reference)))

(event EventTick
  (params (DeltaSeconds :type Float%20%28single-precision%29)))

(fn ConstructionScript)

(fn SaveGame
  (bind _returnvalue (SaveGame|CreateSaveGameObject "/Game/MySaveGame.MySaveGame_C"))
  (Utilities|Array|Clear (Variables|/Game/MySaveGame.MySaveGame_C|GetSavedTransforms _returnvalue))
  (Utilities|Array|Clear (Variables|/Game/MySaveGame.MySaveGame_C|GetCubeVisibility _returnvalue))
  (for _array_element (Variables|Default|GetTrackedCubes)
    (if (Utilities|IsValid _array_element)
      (Utilities|Array|Add (Variables|/Game/MySaveGame.MySaveGame_C|GetSavedTransforms _returnvalue) (Transformation|GetActorTransform _array_element))
      (Utilities|Array|Add (Variables|/Game/MySaveGame.MySaveGame_C|GetCubeVisibility _returnvalue) (Variables|/Script/Engine.Actor|GetbHidden _array_element))))
  (SaveGame|SaveGametoSlot _returnvalue "CubeSaveSlot")
  (bind _returnvalue_2 (SaveGame|DoesSaveGameExist "CubeSaveSlot"))
  (Development|PrintString (Utilities|String|ToString(Boolean) _returnvalue_2)))

(fn LoadGame
  (bind _returnvalue (SaveGame|DoesSaveGameExist "CubeSaveSlot"))
  (if _returnvalue
    (bind _returnvalue_2 (SaveGame|LoadGamefromSlot "CubeSaveSlot"))
    (bind _asmy_save_game (Utilities|Casting|CastToMySaveGame _returnvalue_2))
    (for (_array_element _array_index) (Variables|Default|GetTrackedCubes)
      (if (Utilities|IsValid _array_element)
        (Transformation|SetActorTransform _array_element (Utilities|Array|Get(acopy) (Variables|/Game/MySaveGame.MySaveGame_C|GetSavedTransforms _asmy_save_game) _array_index))
        (Rendering|SetActorHiddenInGame _array_element (Utilities|Array|Get(acopy) (Variables|/Game/MySaveGame.MySaveGame_C|GetCubeVisibility _asmy_save_game) _array_index))))))